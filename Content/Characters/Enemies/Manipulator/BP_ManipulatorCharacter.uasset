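; Manipulator enemy character that handles taking damage and dying.
; AnyDamage reduces health through its Stats component and plays a hurt sound for hits above a small threshold.
; At zero health it plays a death sound, stops the AI brain, starts the death montage, disables collision and destroys itself after a delay.
; IsAudioEnabled gates the whole death sequence, so clearing it also prevents repeat deaths.
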(event `self.ReceiveAnyDamage`
  (params (Damage :type "Float (single-precision)") (DamageType :type "DamageType Object Reference") (InstigatedBy :type "Controller Object Reference") (DamageCauser :type "Actor Object Reference"))
  (bind _mesh (`self.Mesh`))
  (`StatsComponent.ReduceHealth` (`self.Stats`) Damage)
  (if (> Damage 5.0)
    (`GameplayStatics.PlaySoundAtLocation` "/Game/sfx/Corruptor/SFX_Corruptor_Damage.SFX_Corruptor_Damage" (`self.K2_GetActorLocation`) (struct) 1.0 1.0 0.0 null null null null))
  (if (<= (`StatsComponent.GetStat` (`self.Stats`) "Health") 0.0)
    (if (== (`self.IsAudioEnabled`) true)
      (`GameplayStatics.PlaySoundAtLocation` "/Game/sfx/Corruptor/SFX_Corruptor_Death.SFX_Corruptor_Death" (`self.K2_GetActorLocation`) (struct) 1.0 1.0 0.0 null null null null)
      (`BrainComponent.StopLogic` (`AIController.BrainComponent` (`AIBlueprintHelperLibrary.GetAIController` (`PawnMovementComponent.GetPawnOwner` (`self.CharacterMovement`)))) "")
      (`SkeletalMeshComponent.SetAnimationMode` _mesh "AnimationBlueprint" true)
      (`|PlayMontage` _mesh "/Game/Art/Characters/Corruptor/Animations/EyeFix/DeathMontage.DeathMontage" 0.6 0.0 "None" false
        (:`then`
          (`self.SetActorEnableCollision` false)
          (set `self.IsAudioEnabled` false)
          (`KismetSystemLibrary.Delay` 3.5)
          (`self.K2_DestroyActor`))))))

(fn `UserConstructionScript`)